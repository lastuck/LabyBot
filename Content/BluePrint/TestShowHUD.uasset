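; Test actor that creates the WBP_HUD widget and keeps its battery readout in sync with the main camera pawn.
; On BeginPlay it checks that MainCamera is a MainCameraPawn, adds the HUD to the viewport and shows a full battery.
; Tick polls the pawn's RemainingBattery and pushes it to the HUD every frame.
; A minute-and-second timer chain is present but disconnected, so it never runs.
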(event EventBeginPlay
  (bind _asmain_camera_pawn (Utilities|Casting|CastToMainCameraPawn (Variables|Default|GetMainCamera)))
  (bind _returnvalue (UserInterface|CreateWidget "/Game/Widgets/WBP_HUD.WBP_HUD_C"))
  (bind _output_get (Variables|Default|SetHUDRef _returnvalue))
  (UserInterface|Viewport|AddtoViewport _output_get 0)
  (Default|UpdateBattery (Variables|Default|GetHUDRef) 1e+02 1e+02))

(event Collision|EventActorBeginOverlap
  (params (OtherActor :type Actor%20Object%20Reference)))

(event EventTick
  (params (DeltaSeconds :type Float%20%28single-precision%29))
  (bind _asmain_camera_pawn (Utilities|Casting|CastToMainCameraPawn (Variables|Default|GetMainCamera)))
  (Default|UpdateBattery (Variables|Default|GetHUDRef) (Math|Conversions|ToFloat(Integer) (Variables|/Script/MyProject2.MainCameraPawn|GetRemainingBattery _asmain_camera_pawn)) 1e+02))

(fn ConstructionScript)